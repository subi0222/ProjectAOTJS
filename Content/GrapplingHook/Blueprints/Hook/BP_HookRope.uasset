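; BP_HookRope is the visible rope part of a grappling hook, owned by BP_GrapplingHookCharacter.
; SetRopeTransform stretches it between two points by placing it at the start, scaling X by distance and rotating it toward the end.
; On BeginPlay it binds to the character's hook-released event, printing an error if the owner cast fails.
; It destroys itself when the released side matches its IsRight flag.
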(event `self.ReceiveBeginPlay`
  ;[0.3953 0.8899 1] Initialize this rope part on begin play
  (bind _asbp_grappling_hook_character (cast `/Game/GrapplingHook/Blueprints/BP_GrapplingHookCharacter` (`self.GetOwner`))
    (:`then`
      (add `/Game/GrapplingHook/Blueprints/BP_GrapplingHookCharacter.OnHookReleased` _asbp_grappling_hook_character (`|CreateDelegate` :!event `HandleHookReleased`)))
    (:`CastFailed`
      (`KismetSystemLibrary.PrintString` "BP_HookRope: Owner is null or not a BP_GrapplingHookCharacter" true true (struct :`R` 1.0 :`A` 1.0)))))

(event `HandleHookReleased`
  (params (isRight :type Boolean))
  (bind _isright (`self.isRight`))
  ;[1 0.4807 0.2686] Destroy itself when the hook is released
  (if (or (and isRight _isright) (and (not isRight) (not _isright)))
    (`self.K2_DestroyActor`)))

(fn `Set Rope Transform`
  (params (StartLocation :type "Vector Structure (by ref)") (EndLocation :type "Vector Structure (by ref)"))
  (`self.K2_SetActorLocation` StartLocation false true)
  (`self.SetActorScale3D` (`KismetMathLibrary.MakeVector` (/ (`KismetMathLibrary.Vector_Distance` StartLocation EndLocation) 100.0) 0.2 0.2))
  (`self.K2_SetActorRotation` (`KismetMathLibrary.FindLookAtRotation` StartLocation EndLocation) true))

(fn `UserConstructionScript`)