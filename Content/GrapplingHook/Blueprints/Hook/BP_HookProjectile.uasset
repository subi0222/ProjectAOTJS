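; Grappling hook projectile fired by BP_GrapplingHookCharacter for the left or right side, sticking at its hit point and reporting it to the character.
; It spawns a BP_HookRope segment on impact and per new block point, removing one when a point is freed, so the rope bends around terrain.
; Segments realign every tick between hook points and the leg socket.
; On release or no-hit timeout, a timeline lerps it back before cleanup.
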(event `self.ReceiveTick`
  (params (DeltaSeconds :type "Float (single-precision)"))
  ;[0.1818 0.5709 1] Update the rope every tick to get a smooth rope movement when the character moves
  (`self.UpdateRope`)
  ;[1 0.5881 0.3008] Debug
  (bind _asbp_grappling_hook_character (cast `/Game/GrapplingHook/Blueprints/BP_GrapplingHookCharacter` (`self.GetOwner`)))
  (if (`/Game/GrapplingHook/Blueprints/BP_GrapplingHookCharacter.DisplayGrapplingDebug` _asbp_grappling_hook_character)
    (`KismetSystemLibrary.PrintString` (`KismetStringLibrary.Concat_StrStr` (select `bool` (`self.IsRight`) :`false` "Left" :`true` "Right") " hook rope parts: " (`KismetStringLibrary.Conv_IntToString` (`KismetArrayLibrary.Array_Length` (`self.RopeParts`)))) true true (struct :`R` 0.4375 :`G` 0.297082 :`B` 0.136546 :`A` 1.0) 0.0)))

(event `PrematureReturn`
  (bind _ropeparts (`self.RopeParts`))
  ;[1 1 1] Automatically return the projectile because there was no hit.
  (if (not (`self.HookPointFound`))
    (`self.OnReleasedHook`)
    (for _array_element _ropeparts
      (`/Engine/EditorBlueprintResources/StandardMacros.IsValid` _array_element
        (:`Is Valid`
          (`self.K2_DestroyActor` _array_element))))
    (`KismetArrayLibrary.Array_Clear` _ropeparts)))

(event `self.ReceiveBeginPlay`
  ;[0.2322 0.5573 0.4623] Initialize the projectile on BeginPlay
  (`KismetSystemLibrary.K2_SetTimerDelegate` (delegate `PrematureReturn`) (`self.AutoReturnTime`))
  (bind _asbp_grappling_hook_character (cast `/Game/GrapplingHook/Blueprints/BP_GrapplingHookCharacter` (`self.GetOwner`)))
  (add `/Game/GrapplingHook/Blueprints/BP_GrapplingHookCharacter.OnHookBlockPointFound` _asbp_grappling_hook_character (`|CreateDelegate` :!event `HandleNewBlockPoint`))
  (add `/Game/GrapplingHook/Blueprints/BP_GrapplingHookCharacter.OnHookBlockPointFreed` _asbp_grappling_hook_character (`|CreateDelegate` :!event `HandleBlockPointFreed`))
  (set `self.HookRopeWallDistanceRef` (`/Game/GrapplingHook/Blueprints/BP_GrapplingHookCharacter.HookRopeWallDistance` _asbp_grappling_hook_character)))

(event `OnReleasedHook`
  (bind _ropeparts (`self.RopeParts`))
  ;[0.445 0.2421 0.5052] When the hook is called back to the player, we disable the actual projectile movement component and smoothly lerp its position back to the player. Then we destroy the projectile and the player is free to fire it again.
  (if (not (`self.IsReturning`))
    (set `self.IsReturning` true)
    (`ActorComponent.SetActive` (`self.ProjectileMovement`) false false)
    (set `self.TempLocation` (`self.K2_GetActorLocation`))
    (bind _asbp_grappling_hook_character (cast `/Game/GrapplingHook/Blueprints/BP_GrapplingHookCharacter` (`self.GetOwner`)))
    (bind _output_get (set `self.HookLocationsWhenReleased` (select `bool` (`self.isRight`) :`false` (`/Game/GrapplingHook/Blueprints/BP_GrapplingHookCharacter.LeftHookPoints` _asbp_grappling_hook_character) :`true` (`/Game/GrapplingHook/Blueprints/BP_GrapplingHookCharacter.RightHookPoints` _asbp_grappling_hook_character))))
    (if (`self.HookPointFound`)
      (bind _output (`|GetArrayItem` _output_get (`KismetArrayLibrary.Array_LastIndex` _output_get)))
      (`self.K2_SetActorLocation` _output false true)
      (set `self.TempLocation` _output)
      (bind (_direction _alpha) (`Timeline|MoveBackToOwner` :!via `PlayFromStart` :!label _label)
        (:`Update`
          (`self.K2_SetActorLocation` (`KismetMathLibrary.VLerp` (`self.TempLocation`) (`self.K2_GetActorLocation` (`self.GetOwner`)) _alpha)))
        (:`Finished`
          ;[0.932 0.4351 1] Clean-up projectile and rope when the lerp is done.
          (for _array_element _ropeparts
            (`/Engine/EditorBlueprintResources/StandardMacros.IsValid` _array_element
              (:`Is Valid`
                (`self.K2_DestroyActor` _array_element)
                (`KismetArrayLibrary.Array_Remove` _ropeparts))))
          (`self.K2_DestroyActor`)))
      (else
        (goto _label :!via `PlayFromStart`)))))

(event `self.HookCollisionSphere.OnComponentBeginOverlap`
  (params (OverlappedComponent :type "PrimitiveComponent Object Reference") (OtherActor :type "Actor Object Reference") (OtherComp :type "PrimitiveComponent Object Reference") (OtherBodyIndex :type Integer) (bFromSweep :type Boolean) (SweepResult :type "HitResult Structure (by ref)"))
  (bind (_bblockinghit _binitialoverlap _time _distance _location _impactpoint _normal _impactnormal) (`GameplayStatics.BreakHitResult` SweepResult))
  (bind _returnvalue (+ (+ _impactpoint (* _impactnormal (`self.HookRopeWallDistanceRef`))) (* (`self.GetActorForwardVector`) -11.5)))
  ;[0.2719 1 0.1332] The projectile encountered a hit, so we nofity the character, spawn a rope part and adjust the projectile accordingly to stick in the wall.
  (if (and (not (`self.HookPointFound`)) (not (`self.IsReturning`)))
    (set `self.HookPointFound` true)
    (`self.NofityHookLocation` (`self.IsRight`) _returnvalue _impactnormal)
    (`MovementComponent.StopMovementImmediately` (`self.ProjectileMovement`))
    (`self.K2_SetActorLocation` _returnvalue false true)
    (bind _returnvalue_2 (`|SpawnActorFromClass` "/Game/GrapplingHook/Blueprints/Hook/BP_HookRope.BP_HookRope_C" (`KismetMathLibrary.MakeTransform` (0.0 0.0 0.0)) "Undefined" "OverrideRootScale" (`self.GetOwner`) (`self.IsRight`) (`self.GetInstigator`)))
    (`KismetArrayLibrary.Array_AddUnique` (`self.RopeParts`) _returnvalue_2)))

(event `HandleNewBlockPoint`
  (params (NewBlockPoint :type "Vector Structure") (NewBlockPointNormal :type "Vector Structure") (isRight :type Boolean))
  ;[0.7012 1 0.5831] Spawn a new rope for every new hook blocking point. These parts will create the terrain adaptive bending of the rope.
  (bind _returnvalue (`|SpawnActorFromClass` "/Game/GrapplingHook/Blueprints/Hook/BP_HookRope.BP_HookRope_C" (`KismetMathLibrary.MakeTransform` (0.0 0.0 0.0)) "Undefined" "OverrideRootScale" (`self.GetOwner`) isRight (`self.GetInstigator`)))
  (`KismetArrayLibrary.Array_AddUnique` (`self.RopeParts`) _returnvalue)
  (`self.UpdateRope`))

(event `HandleBlockPointFreed`
  (params (isRight :type Boolean))
  (bind _ropeparts (`self.RopeParts`))
  (bind _returnvalue (`KismetArrayLibrary.Array_LastIndex` _ropeparts))
  (bind _output (`|GetArrayItem` _ropeparts _returnvalue))
  ;[1 0.7746 0.6837] Remove a rope part every time a block point is freed
  (`/Engine/EditorBlueprintResources/StandardMacros.IsValid` _output
    (:`Is Valid`
      (`self.K2_DestroyActor` _output))
    (:`Is Not Valid`
      _))
  (`KismetArrayLibrary.Array_Remove` _ropeparts _returnvalue))

(fn `CalculateHookReturnData`
  (params (HookLocationArray :type "Array of Vector Structure"))
  (returns (TotalHookDistance :type "Float (double-precision)") (LastLocationToPlayerDistance :type "Float (double-precision)") (OutHookTravelTimes :type "Array of Float (double-precision)"))
  (locals (InHookInfo :type "Array of Vector Structure") (SumOfDistance :type "Float (double-precision)") (PlayerToLastHookDistance :type "Float (double-precision)") (HookTravelTimes :type "Array of Float (double-precision)"))
  (bind _inhookinfo (`local.InHookInfo`))
  (bind _inhookinfo_2 (`local.InHookInfo`))
  (bind _output_get (set `local.InHookInfo` HookLocationArray))
  (for (_array_element _array_index) _output_get
    (if (>= _array_index 1)
      (set `local.SumOfDistance` (+ (`local.SumOfDistance`) (`KismetMathLibrary.Vector_Distance` _array_element (`|GetArrayItem` _output_get (- _array_index 1)))))))
  (set `local.PlayerToLastHookDistance` (`KismetMathLibrary.Vector_Distance` (`|GetArrayItem` _inhookinfo_2 (`KismetArrayLibrary.Array_LastIndex` _inhookinfo_2)) (`|GetArrayItem` _inhookinfo (- (`KismetArrayLibrary.Array_LastIndex` _inhookinfo) 1))))
  (for (_ _array_index_2) (`local.InHookInfo`)
    (if (>= _array_index_2 1)
      (`KismetArrayLibrary.Array_Add` (`local.HookTravelTimes`))))
  (return (`local.SumOfDistance`) (`local.PlayerToLastHookDistance`) (`local.HookTravelTimes`)))

(fn `NofityHookLocation`
  (params (isRight :type Boolean) (HookLocation :type "Vector Structure") (HookNormal :type "Vector Structure"))
  (bind _asbp_grappling_hook_character (cast `/Game/GrapplingHook/Blueprints/BP_GrapplingHookCharacter` (`self.GetOwner`)))
  (`/Game/GrapplingHook/Blueprints/BP_GrapplingHookCharacter.OnReceiveHookLocation` _asbp_grappling_hook_character isRight HookLocation HookNormal))

(fn `UpdateRope`
  (locals (TempLocations :type "Array of Vector Structure"))
  (bind _returnvalue (`self.GetOwner`))
  (bind _templocations (`local.TempLocations`))
  ;[1 1 1] Update the transform of every rope part for smooth physics
  (if (`self.HookPointFound`)
    (`/Engine/EditorBlueprintResources/StandardMacros.IsValid` _returnvalue
      (:`Is Valid`
        (bind _asbp_grappling_hook_character (cast `/Game/GrapplingHook/Blueprints/BP_GrapplingHookCharacter` _returnvalue))
        (set `self.CharacterAttachLocation` (`SceneComponent.GetSocketLocation` (`Character.Mesh` _asbp_grappling_hook_character) (select `bool` (`self.isRight`) :`false` "LegLeft" :`true` "LegRight" :!type "Name")))
        (set `local.TempLocations` (select `bool` (`self.IsRight`) :`false` (`/Game/GrapplingHook/Blueprints/BP_GrapplingHookCharacter.LeftHookPoints` _asbp_grappling_hook_character) :`true` (`/Game/GrapplingHook/Blueprints/BP_GrapplingHookCharacter.RightHookPoints` _asbp_grappling_hook_character)))
        (`KismetArrayLibrary.Array_Add` (`local.TempLocations`) (`self.CharacterAttachLocation`))
        (for _index (range (+ (- (`KismetArrayLibrary.Array_Length` (`local.TempLocations`)) 2) 1))
          (bind _output (`|GetArrayItem` (`self.RopeParts`) _index))
          (`/Engine/EditorBlueprintResources/StandardMacros.IsValid` _output
            (:`Is Valid`
              (`/Game/GrapplingHook/Blueprints/Hook/BP_HookRope.Set Rope Transform` _output (`|GetArrayItem` _templocations (+ _index 1)) (`|GetArrayItem` _templocations _index)))))))))

(fn `UserConstructionScript`)