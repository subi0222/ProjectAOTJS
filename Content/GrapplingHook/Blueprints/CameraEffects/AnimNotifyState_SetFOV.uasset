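; Anim notify state that eases the grappling hook character's follow camera field of view toward a target during part of an animation.
; Each tick it casts the mesh owner to BP_GrapplingHookCharacter and interpolates FollowCamera's FOV with FInterpTo using the TargetFOV and LerpSpeed variables, skipping the update once within a small tolerance.
; It only defines the tick, so nothing here restores the FOV when the notify ends.
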(fn `Received_NotifyTick`
  (params (MeshComp :type "SkeletalMeshComponent Object Reference") (Animation :type "AnimSequenceBase Object Reference") (FrameDeltaTime :type "Float (single-precision)") (EventReference :type "AnimNotifyEventReference Structure (by ref)"))
  (returns (ReturnValue :type Boolean))
  (bind _asbp_grappling_hook_character (cast `/Game/GrapplingHook/Blueprints/BP_GrapplingHookCharacter` (`ActorComponent.GetOwner` MeshComp)))
  (bind _followcamera (`/Game/GrapplingHook/Blueprints/BP_GrapplingHookCharacter.FollowCamera` _asbp_grappling_hook_character))
  (if (not (`KismetMathLibrary.NearlyEqual_FloatFloat` (`CameraComponent.FieldOfView` _followcamera) (`self.TargetFOV`) 0.1))
    (set `CameraComponent.FieldOfView` (`KismetMathLibrary.FInterpTo` (`CameraComponent.FieldOfView` _followcamera) (`self.TargetFOV`) (`GameplayStatics.GetWorldDeltaSeconds` _followcamera) (`self.LerpSpeed`)) _followcamera)
    (return false)))