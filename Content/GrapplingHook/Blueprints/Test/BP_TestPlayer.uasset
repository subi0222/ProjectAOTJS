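; Test player Blueprint for the grappling hook, handling left and right hook projectiles.
; The fire event spawns a BP_TestProjectile at the given location and rotation, owned and instigated by the player, and stores it per side.
; The release event checks the stored projectile for that side and calls OnReleasedHook on it.
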(event `self.HookProjectileRelease`
  (params (IsRight :type Boolean))
  (bind _righthookprojectile (`self.RightHookProjectile`))
  (bind _lefthookprojectile (`self.LeftHookProjectile`))
  (if IsRight
    (if (`KismetSystemLibrary.IsValid` _righthookprojectile)
      (bind _asbp_test_projectile (cast `/Game/GrapplingHook/Blueprints/Test/BP_TestProjectile` _righthookprojectile))
      (`/Game/GrapplingHook/Blueprints/Test/BP_TestProjectile.OnReleasedHook` _asbp_test_projectile))
    (elif (`KismetSystemLibrary.IsValid` _lefthookprojectile)
      (bind _asbp_test_projectile_2 (cast `/Game/GrapplingHook/Blueprints/Test/BP_TestProjectile` _lefthookprojectile))
      (`/Game/GrapplingHook/Blueprints/Test/BP_TestProjectile.OnReleasedHook` _asbp_test_projectile_2))))

(event `self.HookProjectileFire`
  (params (IsRight :type Boolean) (SpawnLocation :type "Vector Structure") (SpawnRotation :type "Rotator Structure"))
  (if IsRight
    (bind _returnvalue (`|SpawnActorFromClass` "/Game/GrapplingHook/Blueprints/Test/BP_TestProjectile.BP_TestProjectile_C" (`KismetMathLibrary.MakeTransform` SpawnLocation SpawnRotation) "Undefined" "MultiplyWithRoot" self true self))
    (set `self.RightHookProjectile` _returnvalue)
    (else
      (bind _returnvalue_2 (`|SpawnActorFromClass` "/Game/GrapplingHook/Blueprints/Test/BP_TestProjectile.BP_TestProjectile_C" (`KismetMathLibrary.MakeTransform` SpawnLocation SpawnRotation) "Undefined" "MultiplyWithRoot" self false self))
      (set `self.LeftHookProjectile` _returnvalue_2))))

(fn `UserConstructionScript`)